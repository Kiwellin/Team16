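; Camera follow actor that moves its Scene component to track the third-person player character's position.
; BeginPlay caches the player character, and the SetPosition event copies its location to the component while the Follow flag is set.
; The height is held at a hard-coded minimum, so the component stops following the player below that level.
; Nothing in this graph calls SetPosition.
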(event `self.ReceiveBeginPlay`
  (bind _asbp_third_person_character (cast `/Game/BPs/BP_ThirdPersonCharacter` (`GameplayStatics.GetPlayerCharacter` 0)))
  (set `self.Player` _asbp_third_person_character))

(event `SetPosition`
  (bind _returnvalue (- 2250.0 200.0))
  (bind (_returnvalue_x _returnvalue_y _returnvalue_z) (`KismetMathLibrary.BreakVector` (`self.K2_GetActorLocation` (`self.Player`))))
  (if (`self.Follow?`)
    (`SceneComponent.K2_SetWorldLocation` (`self.Scene`) (`KismetMathLibrary.MakeVector` _returnvalue_x _returnvalue_y (`KismetMathLibrary.SelectFloat` _returnvalue _returnvalue_z (< _returnvalue_z _returnvalue))) false false)))

(fn `UserConstructionScript`)