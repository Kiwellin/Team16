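; BP_CamChangeTrigger is a box trigger that switches the player's camera according to the side from which they walk in.
; It caches the player's BP_ThirdPersonCharacter on BeginPlay and reacts only to that actor's overlaps.
; On begin overlap, a dot product of the box's forward vector and the direction to the player picks CamLeave for the front side, otherwise CamEnter, and passes it to ChangeCams.
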(event `self.ReceiveBeginPlay`
  (bind _asbp_third_person_character (cast `/Game/BPs/BP_ThirdPersonCharacter` (`GameplayStatics.GetPlayerPawn` 0)))
  (set `self.Player` _asbp_third_person_character))

(event `self.Box.OnComponentBeginOverlap`
  (params (OverlappedComponent :type "PrimitiveComponent Object Reference") (OtherActor :type "Actor Object Reference") (OtherComp :type "PrimitiveComponent Object Reference") (OtherBodyIndex :type Integer) (bFromSweep :type Boolean) (SweepResult :type "HitResult Structure (by ref)"))
  (bind _player (`self.Player`))
  (if (== OtherActor _player)
    (if (> (`KismetMathLibrary.Dot_VectorVector` (`SceneComponent.GetForwardVector` (`self.Box`)) (`KismetMathLibrary.Normal` (- (`self.K2_GetActorLocation` _player) (`SceneComponent.K2_GetComponentLocation` (`self.Box`))))) 0.0)
      (`/Game/BPs/BP_ThirdPersonCharacter.ChangeCams` (`self.Player`) (`self.CamLeave`))
      (else
        (`/Game/BPs/BP_ThirdPersonCharacter.ChangeCams` (`self.Player`) (`self.CamEnter`))))))

(event `self.Box.OnComponentEndOverlap`
  (params (OverlappedComponent :type "PrimitiveComponent Object Reference") (OtherActor :type "Actor Object Reference") (OtherComp :type "PrimitiveComponent Object Reference") (OtherBodyIndex :type Integer)))

(fn `UserConstructionScript`)