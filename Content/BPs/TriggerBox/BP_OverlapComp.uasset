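; BP_OverlapComp is an overlap component that shows its owner's widget while the player character is inside it.
; On BeginPlay it finds the owner's WidgetComponent and binds its own begin and end overlap events.
; Begin overlap makes the widget visible and end overlap hides it, both only when the other actor casts to BP_ThirdPersonCharacter.
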(event `self.ReceiveBeginPlay`
  (set `self.Widget` (`Actor.GetComponentByClass` (`self.GetOwner`) "/Script/UMG.WidgetComponent"))
  (add `self.OnComponentBeginOverlap` (delegate `OnComponentBeginOverlap_Event`))
  (add `self.OnComponentEndOverlap` (delegate `OverlapEnd`)))

(event `OnComponentBeginOverlap_Event` :!signature `self.OnComponentBeginOverlap`
  (params (OverlappedComponent :type "PrimitiveComponent Object Reference") (OtherActor :type "Actor Object Reference") (OtherComp :type "PrimitiveComponent Object Reference") (OtherBodyIndex :type Integer) (bFromSweep :type Boolean) (SweepResult :type "HitResult Structure (by ref)"))
  (cast `/Game/BPs/BP_ThirdPersonCharacter` OtherActor)
  (`self.SetVisibility` (`self.Widget`) true false))

(event `OverlapEnd` :!signature `self.OnComponentEndOverlap`
  (params (OverlappedComponent :type "PrimitiveComponent Object Reference") (OtherActor :type "Actor Object Reference") (OtherComp :type "PrimitiveComponent Object Reference") (OtherBodyIndex :type Integer))
  (cast `/Game/BPs/BP_ThirdPersonCharacter` OtherActor)
  (`self.SetVisibility` (`self.Widget`) false false))