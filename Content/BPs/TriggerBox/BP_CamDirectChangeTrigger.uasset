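; Trigger box actor that changes the player's camera direction when the player enters it.
; On BeginPlay it casts the player pawn to BP_ThirdPersonCharacter, caches it and prints a debug "Hello".
; When the Box begins overlapping that cached player, it calls CamDirectChange on the character with the trigger's CamRotate value.
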(event `self.ReceiveBeginPlay`
  (bind _asbp_third_person_character (cast `/Game/BPs/BP_ThirdPersonCharacter` (`GameplayStatics.GetPlayerPawn` 0)))
  (set `self.Player` _asbp_third_person_character)
  (`KismetSystemLibrary.PrintString` "Hello"))

(event `self.Box.OnComponentBeginOverlap`
  (params (OverlappedComponent :type "PrimitiveComponent Object Reference") (OtherActor :type "Actor Object Reference") (OtherComp :type "PrimitiveComponent Object Reference") (OtherBodyIndex :type Integer) (bFromSweep :type Boolean) (SweepResult :type "HitResult Structure (by ref)"))
  (if (== OtherActor (`self.Player`))
    (`/Game/BPs/BP_ThirdPersonCharacter.CamDirectChange` (`self.Player`) (`self.CamRotate`))))

(fn `UserConstructionScript`)