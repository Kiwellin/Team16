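; BP_Plank is a one-shot interactable plank that falls into a set rotation when the player interacts with it.
; The first Interact sets InteractWorked, exposed through HasInteracted, and destroys the overlap component and widget so the prompt is gone.
; The PlankFall timeline lerps Scene from its current relative rotation toward TargetRot each update, then plays a 2D wood-drop sound when finished.
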(event `/Game/BPs/Interfaces/BPI_InteractionInterface.Interact`
  (params (Player :type "/Game/BPs/BP_ThirdPersonCharacter Object Reference"))
  (`/Engine/EditorBlueprintResources/StandardMacros.DoOnce` false
    (:`Completed`
      (set `self.InteractWorked` true)
      (`ActorComponent.K2_DestroyComponent` (`self.BP_OverlapComp`))
      (`ActorComponent.K2_DestroyComponent` (`self.Widget`))
      (bind (_direction _alpha) (`Timeline|PlankFall`)
        (:`Update`
          (`SceneComponent.K2_SetRelativeRotation` (`self.Scene`) (`KismetMathLibrary.RLerp` (`SceneComponent.RelativeRotation` (`self.Scene`)) (`self.TargetRot`) _alpha) false false))
        (:`Finished`
          (`GameplayStatics.PlaySound2D` "/Game/Audio/Sfx/ES_Shorts__Drop_On_Wood_-_Epidemic_Sound.ES_Shorts__Drop_On_Wood_-_Epidemic_Sound" 0.8 1.0 0.0 null null))))))

(fn `HasInteracted?`
  (returns (Interact :type Boolean))
  (return (`self.InteractWorked`)))

(fn `UserConstructionScript`)