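; Interactable sink that rises its water level once when used and acts as a hazard for the third-person character.
; Interact disables input, blends the camera to the sink, and shows a temporary cylinder while a timeline lifts Water with sound, then restores view and input.
; Touching Water respawns the character with a drip sound, while the Slippery component launches them backward along the sink's forward axis and upward.
; HasInteracted reports whether it was used.
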(event `self.ReceiveBeginPlay`
  (`SceneComponent.SetHiddenInGame` (`self.Cylinder`) true false))

(event `/Game/BPs/Interfaces/BPI_InteractionInterface.Interact`
  (params (Player :type "/Game/BPs/BP_ThirdPersonCharacter Object Reference"))
  (bind _returnvalue (`GameplayStatics.GetPlayerController` 0))
  (bind _water (`self.Water`))
  (bind (_startloc_x _startloc_y _startloc_z) (`KismetMathLibrary.BreakVector` (`self.StartLoc`)))
  (bind _blend_time (`/Game/BPs/BP_ThirdPersonCharacter.Blend Time` Player))
  (`/Engine/EditorBlueprintResources/StandardMacros.DoOnce` false
    (:`Completed`
      (set `self.InteractWorked` true)
      (`self.DisableInput` (`GameplayStatics.GetPlayerCharacter` 0) _returnvalue)
      (`ActorComponent.K2_DestroyComponent` (`self.Widget`))
      (`ActorComponent.K2_DestroyComponent` (`self.BP_OverlapComp`))
      (`SceneComponent.SetHiddenInGame` (`self.Cylinder`) false false)
      (`PlayerController.SetViewTargetWithBlend` _returnvalue self _blend_time "VTBlend_EaseInOut" 3.0 false)
      (`KismetSystemLibrary.Delay` _blend_time)
      (`GameplayStatics.PlaySoundAtLocation` "/Game/Audio/Sfx/ES_Oral_Rinse__Drinking_From_Faucet_-_Epidemic_Sound_-_4767-8474.ES_Oral_Rinse__Drinking_From_Faucet_-_Epidemic_Sound_-_4767-8474" (`self.K2_GetActorLocation`) (struct) 1.0 1.0 0.0 null null null null)
      (set `self.StartLoc` (`SceneComponent.RelativeLocation` (`self.Water`)))
      (bind (_direction _alpha) (`Timeline|Waterrise`)
        (:`Update`
          (`SceneComponent.K2_SetRelativeLocation` _water (`KismetMathLibrary.VLerp` (`SceneComponent.RelativeLocation` _water) (`KismetMathLibrary.MakeVector` _startloc_x _startloc_y (+ _startloc_z (`self.WaterHeight`))) _alpha) false false))
        (:`Finished`
          (`self.EnableInput` (`GameplayStatics.GetPlayerCharacter` 0) (`GameplayStatics.GetPlayerController` 0))
          (`PlayerController.SetViewTargetWithBlend` (`GameplayStatics.GetPlayerController` 0) (`/Game/BPs/BP_ThirdPersonCharacter.New View Target` Player) (`/Game/BPs/BP_ThirdPersonCharacter.Blend Time` Player) "VTBlend_EaseInOut" 3.0 false)
          (`ActorComponent.K2_DestroyComponent` (`self.Cylinder`)))))))

(event `self.Slippery.OnComponentBeginOverlap`
  (params (OverlappedComponent :type "PrimitiveComponent Object Reference") (OtherActor :type "Actor Object Reference") (OtherComp :type "PrimitiveComponent Object Reference") (OtherBodyIndex :type Integer) (bFromSweep :type Boolean) (SweepResult :type "HitResult Structure (by ref)"))
  (bind _asbp_third_person_character (cast `/Game/BPs/BP_ThirdPersonCharacter` OtherActor))
  (`Character.LaunchCharacter` _asbp_third_person_character (+ (* (`self.GetActorForwardVector`) -2000.0) (0.0 0.0 1200.0)) true true))

(event `self.Water.OnComponentHit`
  (params (HitComponent :type "PrimitiveComponent Object Reference") (OtherActor :type "Actor Object Reference") (OtherComp :type "PrimitiveComponent Object Reference") (NormalImpulse :type "Vector Structure") (Hit :type "HitResult Structure (by ref)"))
  (bind _asbp_third_person_character (cast `/Game/BPs/BP_ThirdPersonCharacter` OtherActor))
  (`/Game/BPs/BP_ThirdPersonCharacter.Respawn` _asbp_third_person_character)
  (`GameplayStatics.PlaySoundAtLocation` "/Game/Audio/Sfx/Waterdrop/SC_WaterDrop.SC_WaterDrop" (`.Location` (`GameplayStatics.BreakHitResult` Hit)) (struct) 1.0 1.0 0.0 null null null null))

(event `self.Water.OnComponentBeginOverlap`
  (params (OverlappedComponent :type "PrimitiveComponent Object Reference") (OtherActor :type "Actor Object Reference") (OtherComp :type "PrimitiveComponent Object Reference") (OtherBodyIndex :type Integer) (bFromSweep :type Boolean) (SweepResult :type "HitResult Structure (by ref)"))
  (bind _asbp_third_person_character (cast `/Game/BPs/BP_ThirdPersonCharacter` OtherActor))
  (`/Game/BPs/BP_ThirdPersonCharacter.Respawn` _asbp_third_person_character)
  (`GameplayStatics.PlaySoundAtLocation` "/Game/Audio/Sfx/Waterdrop/SC_WaterDrop.SC_WaterDrop" (`self.K2_GetActorLocation` _asbp_third_person_character) (struct) 1.0 1.0 0.0 null null null null))

(fn `HasInteracted?`
  (returns (Interact :type Boolean))
  (return (`self.InteractWorked`)))

(fn `UserConstructionScript`)