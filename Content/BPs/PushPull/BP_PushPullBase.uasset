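; Base Blueprint for physics objects that a player can grab to push or pull, optionally restricted by axis.
; On BeginPlay the physics constraint sets its linear limits crosswise: LockY locks X and LockX locks Y, otherwise the axis is free.
; Grab enables physics simulation on the mesh and returns both lock flags to the caller.
; LetGo turns simulation off again.
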(event `self.ReceiveBeginPlay`
  (`PhysicsConstraintComponent.SetLinearXLimit` (`self.PhysicsConstraint`) (select `bool` (`self.LockY`) :`false` "LCM_Free" :`true` "LCM_Locked" :!type "ELinearConstraintMotion Enum") 0.0)
  (`PhysicsConstraintComponent.SetLinearYLimit` (`self.PhysicsConstraint`) (select `bool` (`self.LockX`) :`false` "LCM_Free" :`true` "LCM_Locked" :!type "ELinearConstraintMotion Enum") 0.0))

(event `/Game/BPs/Interfaces/BPI_PushPullObject.LetGo`
  (`PrimitiveComponent.SetSimulatePhysics` (`self.Mesh`) false))

(fn `Grab`
  (params (Player :type "/Game/BPs/BP_ThirdPersonCharacter Object Reference"))
  (returns (LockX :type Boolean) (LockY :type Boolean))
  (`PrimitiveComponent.SetSimulatePhysics` (`self.Mesh`) true)
  (return (`self.LockX`) (`self.LockY`)))

(fn `UserConstructionScript`)